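; Game mode for Toon Tank that handles the start and end presentation of a match through StartGame and GameOver events.
; StartGame shows the start widget, then plays a countdown sound after a short delay.
; GameOver takes a won flag that selects the win or lose sound and sets the end widget's message text and color.
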(event `self.StartGame`
  (bind _returnvalue (`|CreateWidget` "/Game/_Game/Blueprints/UI/WPB_StartGameWidget.WPB_StartGameWidget_C"))
  (`UserWidget.AddToViewport` _returnvalue 0)
  (`KismetSystemLibrary.Delay` 1.5)
  (`GameplayStatics.PlaySound2D` "/Game/Assets/Audio/mixkit-simple-countdown-922.mixkit-simple-countdown-922" 1.0 1.0 0.0 null null))

(event `self.GameOver`
  (params (bWonGame :type Boolean))
  (if bWonGame
    (`GameplayStatics.PlaySound2D` "/Game/Assets/Audio/WinGameSound.WinGameSound" 1.0 1.0 0.0 null null)
    (else
      (`GameplayStatics.PlaySound2D` "/Game/Assets/Audio/GameOverSound.GameOverSound" 1.0 1.0 0.0 null null)))
  (bind _returnvalue (`|CreateWidget` "/Game/_Game/Blueprints/UI/WBP_EndGameWidget.WBP_EndGameWidget_C"))
  (`UserWidget.AddToViewport` _returnvalue 0)
  (bind _displaytext (`/Game/_Game/Blueprints/UI/WBP_EndGameWidget.DisplayText` _returnvalue))
  (`TextBlock.SetText` _displaytext (`KismetTextLibrary.Conv_StringToText` (`KismetMathLibrary.SelectString` "YOU WIN !" "GAME OVER ! " bWonGame)))
  (`TextBlock.SetColorAndOpacity` _displaytext (make `SlateColor` (`KismetMathLibrary.SelectColor` (struct :`R` 0.802083 :`G` 0.469869 :`A` 1.0) (struct :`R` 1.0 :`G` 0.050213 :`A` 1.0) bWonGame))))

(fn `UserConstructionScript`)